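; BP_AIType2 is an AI character variant that shoots once it spots the player or the player base.
; Perception updates run checks for spotting both targets, overriding the parent's perception handling.
; Each tick, if either spot flag is set, it waits out the shoot cooldown through a Delay and then fires a bullet.
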(event `self.ReceiveBeginPlay`
  (`parent.ReceiveBeginPlay`))

(event `self.ReceiveTick`
  (params (DeltaSeconds :type "Float (single-precision)"))
  ; Shootbullet
  (if (or (`self.SpotPlayer?`) (`self.SpotPlayerBase?`))
    (`KismetSystemLibrary.Delay` (`self.ShootCoolDown Duration`))
    (`self.ShootBullet`)))

(event `self.AIPerception.OnPerceptionUpdated`
  (params (UpdatedActors :type "Array of Actor Object Reference (by ref)"))
  ; Overwrite Perception Update
  (`self.checkIfSpotPlayer` UpdatedActors)
  (`self.checkIfSpotBase` UpdatedActors))

(fn `UserConstructionScript`
  (`parent.UserConstructionScript`))