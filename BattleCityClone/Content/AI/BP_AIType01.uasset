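; BP_AIType01 is an enemy AI pawn that shoots, watches for the home base and dies to player bullets.
; A Delay on Tick paces BP_Bullet spawns from ShootingPoint0 to roughly every half second, regardless of target.
; AI Perception updates set the Blackboard's "DetectBase?" flag when a BP_HomeBase appears.
; Capsule hits destroy any bullet, while player bullets also notify BP_ThirdPersonGameMode via DeleteEnemy and destroy the enemy.
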(event `self.ReceiveTick`
  (params (DeltaSeconds :type "Float (single-precision)"))
  ; Shootbullet
  (`KismetSystemLibrary.Delay` 0.5)
  (`self.ShootBullet` :!pinned true) ; Shoot
)

(event `self.AIPerception.OnPerceptionUpdated`
  (params (UpdatedActors :type "Array of Actor Object Reference (by ref)"))
  ; Check if spot base
  (`self.checkIfSpotBase` UpdatedActors))

(event `self.CapsuleComponent.OnComponentHit`
  (params (HitComponent :type "PrimitiveComponent Object Reference") (OtherActor :type "Actor Object Reference") (OtherComp :type "PrimitiveComponent Object Reference") (NormalImpulse :type "Vector Structure") (Hit :type "HitResult Structure (by ref)"))
  ; Hit by bullet
  (bind _asbp_bullet (cast `/Game/Bullet/BP_Bullet` OtherActor))
  (if (`/Game/Bullet/BP_Bullet.isPlayerBullet?` _asbp_bullet)
    (bind _asbp_third_person_game_mode (cast `/Game/ThirdPerson/Blueprints/BP_ThirdPersonGameMode` (`GameplayStatics.GetGameMode`)))
    (`/Game/ThirdPerson/Blueprints/BP_ThirdPersonGameMode.DeleteEnemy` _asbp_third_person_game_mode)
    (`self.K2_DestroyActor`))
  (`/Game/Bullet/BP_Bullet.DestroyBullet` _asbp_bullet))

(fn `checkIfSpotBase`
  (params (ActorLists :type "Array of Actor Object Reference"))
  (for _array_element ActorLists
    ; Spot Base
    (cast `/Game/Tile/BP_HomeBase` _array_element)
    (`BlackboardComponent.SetValueAsBool` (`AIBlueprintHelperLibrary.GetBlackboard` (`AIBlueprintHelperLibrary.GetAIController` self)) "DetectBase?" true)
    (break)))

(fn `ShootBullet`
  (bind (_returnvalue_location _returnvalue_rotation) (`KismetMathLibrary.BreakTransform` (`SceneComponent.K2_GetComponentToWorld` (`self.ShootingPoint_0`))))
  (`|SpawnActorFromClass` "/Game/Bullet/BP_Bullet.BP_Bullet_C" (`KismetMathLibrary.MakeTransform` _returnvalue_location _returnvalue_rotation) "Undefined" "MultiplyWithRoot" null false null))

(fn `UserConstructionScript`)