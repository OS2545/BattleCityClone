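; Mortar-style enemy AI that fires curved BP_Arrow shots at the player or the home base.
; AI perception sets player and base detection flags, mirrored to the Blackboard, with the player taking priority.
; Tick uses a Delay cooldown to fire while a target is spotted, and player respawn clears player detection.
; A player bullet hit kills it with sound and blood effects, notifying the game mode.
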(event `self.ReceiveBeginPlay`
  ; Undetect player when player actor get destroy
  (bind _asbp_third_person_game_mode (cast `/Game/ThirdPerson/Blueprints/BP_ThirdPersonGameMode` (`GameplayStatics.GetGameMode`)))
  (add `/Game/ThirdPerson/Blueprints/BP_ThirdPersonGameMode.ED_Respawn Player` _asbp_third_person_game_mode (delegate `ED_Respawn Player_Event`)))

(event `ED_Respawn Player_Event`
  ; Undetect player when player actor get destroy
  (`self.SetSpotPlayer` false))

(event `self.ReceiveTick`
  (params (DeltaSeconds :type "Float (single-precision)"))
  ; Shootbullet
  (if (or (`self.SpotPlayer?`) (`self.SpotPlayerBase?`))
    (`KismetSystemLibrary.Delay` (`self.shootCoolDownDuration`))
    (`self.ShootMortarBullet` :!pinned true) ; Shoot
  ))

(event `self.AIPerception.OnPerceptionUpdated`
  (params (UpdatedActors :type "Array of Actor Object Reference (by ref)"))
  ; Perception / Task update
  (`self.checkIfSpotPlayer` UpdatedActors)
  (`self.checkIfSpotBase` UpdatedActors))

(event `self.AIPerception.OnTargetPerceptionForgotten`
  (params (Actor :type "Actor Object Reference"))
  ; Perception forgot
  (cast `/Game/ThirdPerson/Blueprints/BP_ThirdPersonCharacter` Actor
    (:`then`
      (`self.SetSpotPlayer` false))
    (:`CastFailed`
      (cast `/Game/Tile/BP_HomeBase` Actor)
      (`self.SetSpotPlayerBase` false))))

(event `self.CapsuleComponent.OnComponentHit`
  (params (HitComponent :type "PrimitiveComponent Object Reference") (OtherActor :type "Actor Object Reference") (OtherComp :type "PrimitiveComponent Object Reference") (NormalImpulse :type "Vector Structure") (Hit :type "HitResult Structure (by ref)"))
  ; Hit by bullet
  (bind _asbp_arrow (cast `/Game/Bullet/BP_Arrow` OtherActor))
  (if (`/Game/Bullet/BP_Arrow.isPlayerBullet?` _asbp_arrow)
    (`self.AIIsDestroyed` _asbp_arrow)))

(fn `AIIsDestroyed`
  (params (Bullet :type "/Game/Bullet/BP_Arrow Object Reference"))
  (`/Engine/EditorBlueprintResources/StandardMacros.IsValid` Bullet
    (:`Is Valid`
      (`/Game/Bullet/BP_Arrow.BulletHit` Bullet)
      (`GameplayStatics.PlaySoundAtLocation` "/Game/SoundEffect/SW_arrow_body_impact.SW_arrow_body_impact" (`self.K2_GetActorLocation`) (struct) 1.0 1.0 0.0 null null null null)
      (`NiagaraFunctionLibrary.SpawnSystemAtLocation` "/Game/VFX/BloodSplatter/NS_BloodSplatter.NS_BloodSplatter" (`self.K2_GetActorLocation` self))
      (bind _asbp_third_person_game_mode (cast `/Game/ThirdPerson/Blueprints/BP_ThirdPersonGameMode` (`GameplayStatics.GetGameMode`)))
      (`/Game/ThirdPerson/Blueprints/BP_ThirdPersonGameMode.DestroyEnemy` _asbp_third_person_game_mode)
      (`self.K2_DestroyActor`))))

(fn `checkIfSpotBase`
  (params (`Actor List` :type "Array of Actor Object Reference"))
  (locals (`spotBase?` :type Boolean))
  (if (`self.SpotPlayer?`)
    ; Priority Player
    (`self.SetSpotPlayerBase` false)
    (else
      (for _array_element `Actor List`
        ; Spot Base
        (cast `/Game/Tile/BP_HomeBase` _array_element)
        (`self.SetSpotPlayerBase` true)
        (break)))))

(fn `checkIfSpotPlayer`
  (params (ActorLists :type "Array of Actor Object Reference"))
  (for _array_element ActorLists
    ; Spot Player
    (`/Engine/EditorBlueprintResources/StandardMacros.IsValid` _array_element
      (:`Is Valid`
        (cast `/Game/ThirdPerson/Blueprints/BP_ThirdPersonCharacter` _array_element)
        (`self.SetSpotPlayer` true)
        (break)))))

(fn `SetSpotPlayer`
  (params (`spotPlayer?` :type Boolean))
  (`BlackboardComponent.SetValueAsBool` (`AIBlueprintHelperLibrary.GetBlackboard` (`AIBlueprintHelperLibrary.GetAIController` self)) "DetectPlayer?" `spotPlayer?`)
  (set `self.SpotPlayer?` `spotPlayer?`))

(fn `SetSpotPlayerBase`
  (params (`spotBase?` :type Boolean))
  (`BlackboardComponent.SetValueAsBool` (`AIBlueprintHelperLibrary.GetBlackboard` (`AIBlueprintHelperLibrary.GetAIController` self)) "DetectBase?" `spotBase?`)
  (set `self.SpotPlayerBase?` `spotBase?`))

(fn `ShootMortarBullet`
  (bind _returnvalue_location (`KismetMathLibrary.BreakTransform` (`SceneComponent.K2_GetComponentToWorld` (`self.ShootingPoint_0`))))
  (if (`self.SpotPlayer?`)
    (bind _asbp_third_person_character (cast `/Game/ThirdPerson/Blueprints/BP_ThirdPersonCharacter` (`GameplayStatics.GetPlayerPawn` 0)))
    (`/Engine/EditorBlueprintResources/StandardMacros.IsValid` _asbp_third_person_character
      (:`Is Valid`
        (`|SpawnActorFromClass` "/Game/Bullet/BP_Arrow.BP_Arrow_C" (`KismetMathLibrary.MakeTransform` _returnvalue_location) "Undefined" "MultiplyWithRoot" null false true _asbp_third_person_character null)))
    (elif (`self.SpotPlayerBase?`)
      (bind _returnvalue (`GameplayStatics.GetActorOfClass` "/Game/Tile/BP_HomeBase.BP_HomeBase_C"))
      (`|SpawnActorFromClass` "/Game/Bullet/BP_Arrow.BP_Arrow_C" (`KismetMathLibrary.MakeTransform` _returnvalue_location) "Undefined" "MultiplyWithRoot" null false true _returnvalue null))))

(fn `UserConstructionScript`)