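; Enemy AI character that fires arrows on a repeating Tick-plus-Delay cooldown, regardless of target.
; AI perception flags the home base unless the player is spotted, updating blackboard booleans and current target; the player-spotting function is never called here.
; Forgotten targets and the game mode's player-respawn dispatcher clear detection.
; Player arrow hits notify the game mode and destroy it with sound and blood effects.
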(event `self.ReceiveBeginPlay`
  ; Undetect player when player actor get destroy
  (bind _asbp_third_person_game_mode (cast `/Game/ThirdPerson/Blueprints/BP_ThirdPersonGameMode` (`GameplayStatics.GetGameMode`)))
  (add `/Game/ThirdPerson/Blueprints/BP_ThirdPersonGameMode.ED_Respawn Player` _asbp_third_person_game_mode (delegate `ED_Respawn Player_Event`)))

(event `ED_Respawn Player_Event`
  ; Undetect player when player actor get destroy
  (`self.SetSpotPlayer` false))

(event `self.ReceiveTick`
  (params (DeltaSeconds :type "Float (single-precision)"))
  ; Shootbullet
  (`KismetSystemLibrary.Delay` (`self.ShootCoolDown Duration`))
  (`self.ShootBullet` :!pinned true) ; Shoot
)

(event `self.AIPerception.OnPerceptionUpdated`
  (params (UpdatedActors :type "Array of Actor Object Reference (by ref)"))
  ; Check if spot base
  (`self.checkIfSpotBase` UpdatedActors))

(event `self.AIPerception.OnTargetPerceptionForgotten`
  (params (Actor :type "Actor Object Reference"))
  ; Perception forgot
  (cast `/Game/ThirdPerson/Blueprints/BP_ThirdPersonCharacter` Actor
    (:`then`
      (`self.SetSpotPlayer` false))
    (:`CastFailed`
      (cast `/Game/Tile/BP_HomeBaseTile` Actor)
      (`self.SetSpotPlayerBase` false))))

(event `self.CapsuleComponent.OnComponentHit`
  (params (HitComponent :type "PrimitiveComponent Object Reference") (OtherActor :type "Actor Object Reference") (OtherComp :type "PrimitiveComponent Object Reference") (NormalImpulse :type "Vector Structure") (Hit :type "HitResult Structure (by ref)"))
  ; Hit by bullet
  (`self.checkIfHit` OtherActor))

(event `self.ReceiveDestroyed`
  (`GameplayStatics.PlaySoundAtLocation` "/Game/SoundEffect/SC_CharacterGetHit.SC_CharacterGetHit" (`self.K2_GetActorLocation`) (struct) 1.0 1.0 0.0 null null null null)
  (`NiagaraFunctionLibrary.SpawnSystemAtLocation` "/Game/VFX/BloodSplatter/NS_BloodSplatter.NS_BloodSplatter" (`self.K2_GetActorLocation` self)))

(fn `AIIsDestroyed`
  (params (Bullet :type "/Game/Bullet/BP_Arrow Object Reference"))
  (`/Engine/EditorBlueprintResources/StandardMacros.IsValid` Bullet
    (:`Is Valid`
      (`/Game/Bullet/BP_Arrow.BulletHit` Bullet)
      (bind _asbp_third_person_game_mode (cast `/Game/ThirdPerson/Blueprints/BP_ThirdPersonGameMode` (`GameplayStatics.GetGameMode`)))
      (`/Game/ThirdPerson/Blueprints/BP_ThirdPersonGameMode.DestroyEnemy` _asbp_third_person_game_mode)
      (`self.K2_DestroyActor`))))

(fn `checkIfHit`
  (params (otherActor :type "Actor Object Reference"))
  (bind _asbp_arrow (cast `/Game/Bullet/BP_Arrow` otherActor))
  (if (`/Game/Bullet/BP_Arrow.isPlayerBullet?` _asbp_arrow)
    (`self.AIIsDestroyed` _asbp_arrow)
    (else
      (`/Game/Bullet/BP_Arrow.BulletHit` _asbp_arrow))))

(fn `checkIfSpotBase`
  (params (ActorLists :type "Array of Actor Object Reference"))
  (if (`self.SpotPlayer?`)
    (`self.SetSpotPlayerBase` false)
    (else
      (for _array_element ActorLists
        (cast `/Game/Tile/BP_HomeBaseTile` _array_element)
        (`self.SetSpotPlayerBase` true)
        (break)))))

(fn `checkIfSpotPlayer`
  (params (ActorLists :type "Array of Actor Object Reference"))
  (locals (_playerspot :type Boolean))
  (for _array_element ActorLists
    ; Spot Player
    (cast `/Game/ThirdPerson/Blueprints/BP_ThirdPersonCharacter` _array_element)
    (`self.SetSpotPlayer` true)
    (break)))

(fn `SetSpotPlayer`
  (params (`spotPlayer?` :type Boolean))
  (`BlackboardComponent.SetValueAsBool` (`AIBlueprintHelperLibrary.GetBlackboard` (`AIBlueprintHelperLibrary.GetAIController` self)) "DetectPlayer?" `spotPlayer?`)
  (bind _output_get (set `self.SpotPlayer?` `spotPlayer?`))
  (if _output_get
    (set `self.currentTarget` (`GameplayStatics.GetPlayerPawn` 0))))

(fn `SetSpotPlayerBase`
  (params (`spotBase?` :type Boolean))
  (`BlackboardComponent.SetValueAsBool` (`AIBlueprintHelperLibrary.GetBlackboard` (`AIBlueprintHelperLibrary.GetAIController` self)) "DetectBase?" `spotBase?`)
  (bind _output_get (set `self.SpotPlayerBase?` `spotBase?`))
  (if _output_get
    (bind _returnvalue (`GameplayStatics.GetActorOfClass` "/Game/Tile/BP_HomeBaseTile.BP_HomeBaseTile_C"))
    (set `self.currentTarget` _returnvalue)))

(fn `ShootBullet`
  (bind (_returnvalue_location _returnvalue_rotation) (`KismetMathLibrary.BreakTransform` (`SceneComponent.K2_GetComponentToWorld` (`self.ShootingPoint_0`))))
  (`|SpawnActorFromClass` "/Game/Bullet/BP_Arrow.BP_Arrow_C" (`KismetMathLibrary.MakeTransform` _returnvalue_location _returnvalue_rotation) "Undefined" "MultiplyWithRoot" null false null))

(fn `UserConstructionScript`)