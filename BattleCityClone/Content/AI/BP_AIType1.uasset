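; BP_AIType1 is an AI shooter that fires automatically and repeatedly, with no targeting or movement logic in its graphs.
; Each Tick either counts down the cooldown or, once it has expired, calls ShootBullet.
; ShootBullet spawns BP_Bullet at the ShootingPoint0 transform and restarts the cooldown from MAXCOOLDOWN.
; The countdown subtracts a fixed step per frame rather than using delta time, so fire rate depends on frame rate.
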(event `self.ReceiveBeginPlay`
  ; Assign shooting cool down
  (set `self.coolDownTime` (`self.MAX_COOLDOWN`)))

(event `self.ReceiveTick`
  (params (DeltaSeconds :type "Float (single-precision)"))
  (if (`self.shootCoolDown`)
    ; Cool down
    (bind _output_get (set `self.coolDownTime` (- (`self.coolDownTime`) 0.1)))
    (if (<= _output_get 0.0)
      (set `self.shootCoolDown` false))
    (else
      (`self.ShootBullet` :!pinned true) ; Shoot
    )))

(fn `ShootBullet`
  (bind (_returnvalue_location _returnvalue_rotation) (`KismetMathLibrary.BreakTransform` (`SceneComponent.K2_GetComponentToWorld` (`self.ShootingPoint_0`))))
  (set `self.shootCoolDown` true)
  (set `self.coolDownTime` (`self.MAX_COOLDOWN`))
  (`|SpawnActorFromClass` "/Game/Bullet/BP_Bullet.BP_Bullet_C" (`KismetMathLibrary.MakeTransform` _returnvalue_location _returnvalue_rotation) "Undefined" "MultiplyWithRoot" null false null))

(fn `UserConstructionScript`)