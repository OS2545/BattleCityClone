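; BP_AIType3 is a ranged enemy AI that fires curve arrows at the player or the home base.
; Perception updates call inherited-style checks for spotting either target.
; While either is spotted, Tick feeds a cooldown Delay that throttles shooting.
; Each shot spawns a BP_CurveArrow at the shooting point, targeting the player first and otherwise the BP_HomeBaseTile actor.
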(event `self.ReceiveBeginPlay`
  (`parent.ReceiveBeginPlay`)
  (set `self.ShootCoolDown Duration` 1.0))

(event `self.ReceiveTick`
  (params (DeltaSeconds :type "Float (single-precision)"))
  ; Shootbullet
  (if (or (`self.SpotPlayer?`) (`self.SpotPlayerBase?`))
    (`KismetSystemLibrary.Delay` (`self.ShootCoolDown Duration`))
    (`self.ShootBullet`)))

(event `self.AIPerception.OnPerceptionUpdated`
  (params (UpdatedActors :type "Array of Actor Object Reference (by ref)"))
  ; Overwrite Perception Update
  (`self.checkIfSpotPlayer` UpdatedActors)
  (`self.checkIfSpotBase` UpdatedActors))

(event `self.ShootBullet`
  (bind _returnvalue_location (`KismetMathLibrary.BreakTransform` (`SceneComponent.K2_GetComponentToWorld` (`self.ShootingPoint_0`))))
  (if (`self.SpotPlayer?`)
    (bind _asbp_third_person_character (cast `/Game/ThirdPerson/Blueprints/BP_ThirdPersonCharacter` (`GameplayStatics.GetPlayerPawn` 0)))
    (`/Engine/EditorBlueprintResources/StandardMacros.IsValid` _asbp_third_person_character
      (:`Is Valid`
        (`|SpawnActorFromClass` "/Game/Bullet/BP_CurveArrow.BP_CurveArrow_C" (`KismetMathLibrary.MakeTransform` _returnvalue_location) "Undefined" "MultiplyWithRoot" null _asbp_third_person_character false null)))
    (elif (`self.SpotPlayerBase?`)
      (bind _returnvalue (`GameplayStatics.GetActorOfClass` "/Game/Tile/BP_HomeBaseTile.BP_HomeBaseTile_C"))
      (`|SpawnActorFromClass` "/Game/Bullet/BP_CurveArrow.BP_CurveArrow_C" (`KismetMathLibrary.MakeTransform` _returnvalue_location) "Undefined" "MultiplyWithRoot" null _returnvalue false null))))

(fn `UserConstructionScript`
  (`parent.UserConstructionScript`))