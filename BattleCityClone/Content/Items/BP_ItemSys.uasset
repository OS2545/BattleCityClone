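; Item system actor that tracks whether the player holds one special ammo charge (special arrow) and one armor charge.
; Add functions refuse duplicates and play a gain sound; adding armor also spawns BP_ArmorItem attached to the player, using the character's relative scale as location.
; Use functions clear the flag, with UseArmor also firing the EDUseArmor dispatcher.
; State changes are pushed to the UI through HUD_UI.
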(fn `AddArmor`
  (returns (`add Sucess?` :type Boolean))
  (bind _returnvalue (`GameplayStatics.GetPlayerPawn` 0))
  (if (not (`self.armor?`))
    (`/Engine/EditorBlueprintResources/StandardMacros.IsValid` _returnvalue
      (:`Is Valid`
        ; Add armor visual and sound when gaining armor
        (bind _asbp_third_person_character (cast `/Game/ThirdPerson/Blueprints/BP_ThirdPersonCharacter` _returnvalue))
        (bind _returnvalue_2 (`self.GetActorRelativeScale3D` _asbp_third_person_character))
        (bind _returnvalue_3 (`|SpawnActorFromClass` "/Game/Items/BP_ArmorItem.BP_ArmorItem_C" (`KismetMathLibrary.MakeTransform` _returnvalue_2) "Undefined" "MultiplyWithRoot" null null))
        (`self.K2_AttachToActor` _returnvalue_3 _returnvalue "None" "KeepRelative" "KeepRelative" "KeepRelative" true)
        (`GameplayStatics.PlaySoundAtLocation` "/Game/SoundEffect/SW_Items/SW_armorGain.SW_armorGain" _returnvalue_2 (struct) 1.0 1.0 0.0 null null null null)
        (set `self.armor?` true)
        (`self.UpdateArmorVisualUI`)
        (return true))
      (:`Is Not Valid`
        _)))
  (return false))

(fn `AddSpecialAmmo`
  (returns (`Add Sucess?` :type Boolean))
  (bind _returnvalue (`GameplayStatics.GetPlayerPawn` 0))
  (if (`self.specialAmmo?`)
    (return false)
    (else
      (set `self.specialAmmo?` true)
      ; Add sound when gain special arrow
      (`/Engine/EditorBlueprintResources/StandardMacros.IsValid` _returnvalue
        (:`Is Valid`
          (bind _asbp_third_person_character (cast `/Game/ThirdPerson/Blueprints/BP_ThirdPersonCharacter` _returnvalue))
          (`GameplayStatics.PlaySoundAtLocation` "/Game/SoundEffect/SW_Items/SW_specialArrowGain.SW_specialArrowGain" (`self.GetActorRelativeScale3D` _asbp_third_person_character) (struct) 1.0 1.0 0.0 null null null null)
          (`self.UpdateSpecialBulletVisualUI`)
          (return true))))))

(fn `HasArmor`
  (returns (`hasArmor?` :type Boolean))
  (return (`self.armor?`)))

(fn `HasSpecialAmmo`
  (returns (`has special ammo?` :type Boolean))
  (return (`self.specialAmmo?`)))

(fn `UpdateArmorVisualUI`
  (bind _ashud_ui (cast `/Game/UI/HUD_UI` (`PlayerController.GetHUD` (`GameplayStatics.GetPlayerController` 0))))
  (`/Game/UI/W_UI.UpdateArmorUI_Event` (`/Game/UI/HUD_UI.UI_Ref` _ashud_ui) (`self.armor?`)))

(fn `UpdateSpecialBulletVisualUI`
  (bind _ashud_ui (cast `/Game/UI/HUD_UI` (`PlayerController.GetHUD` (`GameplayStatics.GetPlayerController` 0))))
  (`/Game/UI/W_UI.UpdateSpecialBullet_Event` (`/Game/UI/HUD_UI.UI_Ref` _ashud_ui) (`self.specialAmmo?`)))

(fn `UseArmor`
  (set `self.armor?` false)
  (`self.ED_UseArmor`)
  (`self.UpdateArmorVisualUI`)
  (return))

(fn `UserConstructionScript`)

(fn `UseSpecialAmmo`
  (set `self.specialAmmo?` false)
  (`self.UpdateSpecialBulletVisualUI`)
  (return))