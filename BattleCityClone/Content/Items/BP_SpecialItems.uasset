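; BP_SpecialItems is a pickup actor that grants either special ammo or armor, chosen by the AmmoOrArmor boolean (true means ammo).
; On BeginPlay it shows the matching bullet or armor mesh.
; When BP_ThirdPersonCharacter overlaps Mesh_bullet, the only bound overlap trigger, it calls AddSpecialAmmo or AddArmor on BP_ThirdPersonGameMode.
; It destroys itself only if that call reports success.
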(event `self.ReceiveBeginPlay`
  (`self.AssignModel`))

(event `self.Mesh_bullet.OnComponentBeginOverlap`
  (params (OverlappedComponent :type "PrimitiveComponent Object Reference") (OtherActor :type "Actor Object Reference") (OtherComp :type "PrimitiveComponent Object Reference") (OtherBodyIndex :type Integer) (bFromSweep :type Boolean) (SweepResult :type "HitResult Structure (by ref)"))
  (cast `/Game/ThirdPerson/Blueprints/BP_ThirdPersonCharacter` OtherActor)
  (`self.AddItemToInventory`))

(fn `AddItemToInventory`
  (locals (BP_Player :type "/Game/ThirdPerson/Blueprints/BP_ThirdPersonCharacter Object Reference"))
  (bind _asbp_third_person_game_mode (cast `/Game/ThirdPerson/Blueprints/BP_ThirdPersonGameMode` (`GameplayStatics.GetGameMode`)))
  (if (`self.AmmoOrArmor`)
    (bind _add_sucess_ (`/Game/ThirdPerson/Blueprints/BP_ThirdPersonGameMode.AddSpecialAmmo` _asbp_third_person_game_mode))
    (if _add_sucess_
      (`self.K2_DestroyActor`))
    (else
      (bind _add_sucess__2 (`/Game/ThirdPerson/Blueprints/BP_ThirdPersonGameMode.AddArmor` _asbp_third_person_game_mode))
      (if _add_sucess__2
        (`self.K2_DestroyActor`)))))

(fn `AssignModel`
  (if (`self.AmmoOrArmor`)
    (`SceneComponent.SetVisibility` (`self.Mesh_bullet`) true false)
    (else
      (`SceneComponent.SetVisibility` (`self.Mesh_armor`) true false)))
  (return))

(fn `UserConstructionScript`)