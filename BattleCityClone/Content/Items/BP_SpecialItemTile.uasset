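; BP_SpecialItemTile is a pickup actor that gives the player either special ammo or armor, chosen by the AmmoOrArmor flag.
; On BeginPlay it shows the bullet or armor mesh to match the flag.
; A player overlap with the bullet mesh, which triggers both pickup types, calls the matching add function on BP_ItemSys, found via GetActorOfClass.
; The tile destroys itself only if that call succeeds.
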(event `self.ReceiveBeginPlay`
  (`self.AssignModel`))

(event `self.Mesh_bullet.OnComponentBeginOverlap`
  (params (OverlappedComponent :type "PrimitiveComponent Object Reference") (OtherActor :type "Actor Object Reference") (OtherComp :type "PrimitiveComponent Object Reference") (OtherBodyIndex :type Integer) (bFromSweep :type Boolean) (SweepResult :type "HitResult Structure (by ref)"))
  ; Check if it is player
  (cast `/Game/ThirdPerson/Blueprints/BP_ThirdPersonCharacter` OtherActor)
  (`self.AddItemToInventory`))

(fn `AddItemToInventory`
  (locals (BP_Player :type "/Game/ThirdPerson/Blueprints/BP_ThirdPersonCharacter Object Reference"))
  (bind _returnvalue (`GameplayStatics.GetActorOfClass` "/Game/Items/BP_ItemSys.BP_ItemSys_C"))
  (if (`self.AmmoOrArmor`)
    (bind _add_sucess_ (`/Game/Items/BP_ItemSys.AddSpecialAmmo` _returnvalue))
    (if _add_sucess_
      (`self.K2_DestroyActor`))
    (else
      (bind _add_sucess__2 (`/Game/Items/BP_ItemSys.AddArmor` _returnvalue))
      (if _add_sucess__2
        (`self.K2_DestroyActor`)))))

(fn `AssignModel`
  (if (`self.AmmoOrArmor`)
    (`SceneComponent.SetVisibility` (`self.Mesh_bullet`) true false)
    (else
      (`SceneComponent.SetVisibility` (`self.Mesh_armor`) true false)))
  (return))

(fn `UserConstructionScript`)