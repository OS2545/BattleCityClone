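; Arrow projectile that flies straight or arcs toward a target, with a 10-second lifetime via a Tick delay.
; Curve arrows lead the target by its velocity and distance using SuggestProjectileVelocityCustomArc, then enable gravity.
; Player arrows with special ammo from BP_ItemSys start as overlap to pierce one wall tile, then restore blocking and spend the ammo.
; Hitting another arrow plays an impact sound, fires a radial impulse and destroys it.
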(event `self.ReceiveBeginPlay`
  ; Play release arrow sound
  (`GameplayStatics.PlaySoundAtLocation` "/Game/SoundEffect/SW_Arrow/SW_ArrowRelease.SW_ArrowRelease" (`self.K2_GetActorLocation` self) (struct) 1.0 1.0 0.0 null null null null)
  ; Manage curve arrow
  (if (`self.isCurveArrow`)
    (`/Engine/EditorBlueprintResources/StandardMacros.IsValid` (`self.curveArrowTarget`)
      (:`Is Valid`
        (`self.SetCurveArrow`))
      (:`Is Not Valid`
        (`self.K2_DestroyActor`)))
    (else
      ; Check if has special bullet
      (if (`self.isPlayerBullet?`)
        (bind _returnvalue (`GameplayStatics.GetActorOfClass` "/Game/Items/BP_ItemSys.BP_ItemSys_C"))
        (bind _has_special_ammo_ (`/Game/Items/BP_ItemSys.HasSpecialAmmo` _returnvalue))
        (if _has_special_ammo_
          (`PrimitiveComponent.SetCollisionResponseToAllChannels` (`self.SphereCollision`) "ECR_Overlap"))))))

(event `self.SphereCollision.OnComponentBeginOverlap`
  (params (OverlappedComponent :type "PrimitiveComponent Object Reference") (OtherActor :type "Actor Object Reference") (OtherComp :type "PrimitiveComponent Object Reference") (OtherBodyIndex :type Integer) (bFromSweep :type Boolean) (SweepResult :type "HitResult Structure (by ref)"))
  ; Check other thing than BP_Destrucible/Indestrucible wall. The bullet return to normal collision
  (`/Engine/EditorBlueprintResources/StandardMacros.IsValid` OtherActor
    (:`Is Valid`
      (cast `/Game/Tile/BP_DestructibleTile` OtherActor
        (:`then`
          (set `self.isSpecialbulletIsUsed?` true :!label _label))
        (:`CastFailed`
          (cast `/Game/Tile/BP_IndestructibleWallTile` OtherActor
            (:`then`
              (goto _label))
            (:`CastFailed`
              ;; If not pass thought the wall then return to normal collision
              (`PrimitiveComponent.SetCollisionResponseToAllChannels` (`self.SphereCollision`) "ECR_Block" :!label _label_2))))))
    (:`Is Not Valid`
      (goto _label_2))))

(event `self.SphereCollision.OnComponentEndOverlap`
  (params (OverlappedComponent :type "PrimitiveComponent Object Reference") (OtherActor :type "Actor Object Reference") (OtherComp :type "PrimitiveComponent Object Reference") (OtherBodyIndex :type Integer))
  ; Has special bullet => pass throught a wall / Use special Bullet
  (if (`self.isSpecialbulletIsUsed?`)
    (`PrimitiveComponent.SetCollisionResponseToAllChannels` (`self.SphereCollision`) "ECR_Block")
    (if (`self.isPlayerBullet?`)
      (bind _returnvalue (`GameplayStatics.GetActorOfClass` "/Game/Items/BP_ItemSys.BP_ItemSys_C"))
      (`/Game/Items/BP_ItemSys.UseSpecialAmmo` _returnvalue))))

(event `self.SphereCollision.OnComponentHit`
  (params (HitComponent :type "PrimitiveComponent Object Reference") (OtherActor :type "Actor Object Reference") (OtherComp :type "PrimitiveComponent Object Reference") (NormalImpulse :type "Vector Structure") (Hit :type "HitResult Structure (by ref)"))
  ; Hit Something
  (`/Engine/EditorBlueprintResources/StandardMacros.IsValid` OtherActor
    (:`Is Valid`
      ;; Check if bullet
      (cast `/Game/Bullet/BP_Arrow` OtherActor)
      (`GameplayStatics.PlaySoundAtLocation` "/Game/SoundEffect/SW_Arrow/SW_arrow_arrow_impact.SW_arrow_arrow_impact" (`self.K2_GetActorLocation`) (struct) 1.0 1.0 0.0 null null null null))
    (:`Is Not Valid`
      _))
  (`self.BulletHit`))

(event `self.ReceiveTick`
  (params (DeltaSeconds :type "Float (single-precision)"))
  ; After 10 second bullet automatically destroy
  (`KismetSystemLibrary.Delay` 10.0)
  (`self.K2_DestroyActor`))

(fn `BulletHit`
  ; Manage Emitter
  (`RadialForceComponent.FireImpulse` (`self.RadialForce`))
  (`self.K2_DestroyActor`))

(fn `CalculateCurveTargetVelocity`
  (returns (Velocity :type "Vector Structure"))
  (locals (TargetActorVelocity :type "Vector Structure") (TargetActorLocation :type "Vector Structure") (Arc :type "Float (double-precision)" :default 1200.0))
  (bind _curvearrowtarget (`self.curveArrowTarget`))
  (set `local.TargetActorVelocity` (`self.GetVelocity` _curvearrowtarget))
  (set `local.TargetActorLocation` (`self.K2_GetActorLocation` _curvearrowtarget))
  (bind (_outlaunchvelocity _returnvalue) (`GameplayStatics.SuggestProjectileVelocity_CustomArc` (`self.K2_GetActorLocation`) (+ (`local.TargetActorLocation`) (* (`local.TargetActorVelocity`) (/ (`KismetMathLibrary.Vector_Distance` (`local.TargetActorLocation`) (`self.K2_GetActorLocation`)) (`KismetSystemLibrary.MakeLiteralDouble` (`local.Arc`)))))))
  (if _returnvalue
    (return _outlaunchvelocity)))

(fn `SetCurveArrow`
  (bind _projectilemovement (`self.ProjectileMovement`))
  (bind _velocity (`self.CalculateCurveTargetVelocity`))
  (`ProjectileMovementComponent.SetVelocityInLocalSpace` (`self.ProjectileMovement`) _velocity)
  (set `ProjectileMovementComponent.bInterpMovement` true _projectilemovement)
  (set `ProjectileMovementComponent.ProjectileGravityScale` 1.0 _projectilemovement))

(fn `UserConstructionScript`)