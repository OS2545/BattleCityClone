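; Mortar projectile that lobs itself at a Target actor and explodes on impact, destroying itself at spawn if no target is valid.
; On BeginPlay it leads the target by its velocity times distance divided by Arc, then feeds SuggestProjectileVelocityCustomArc's result to ProjectileMovement as a local-space velocity.
; A collision sphere hit fires a radial force impulse, spawns an explosion particle and destroys the bullet.
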(event `self.ReceiveBeginPlay`
  (`/Engine/EditorBlueprintResources/StandardMacros.IsValid` (`self.Target`)
    (:`Is Valid`
      (bind _velocity (`self.CalculateMortarVelocity`))
      (`ProjectileMovementComponent.SetVelocityInLocalSpace` (`self.ProjectileMovement`) _velocity))
    (:`Is Not Valid`
      (`self.K2_DestroyActor`))))

(event `self.CollisionSphere.OnComponentHit`
  (params (HitComponent :type "PrimitiveComponent Object Reference") (OtherActor :type "Actor Object Reference") (OtherComp :type "PrimitiveComponent Object Reference") (NormalImpulse :type "Vector Structure") (Hit :type "HitResult Structure (by ref)"))
  (bind _returnvalue_location (`KismetMathLibrary.BreakTransform` (`SceneComponent.GetRelativeTransform` (`self.CollisionSphere`))))
  ; On bullet Hit
  (`RadialForceComponent.FireImpulse` (`self.RadialForce`))
  (`GameplayStatics.SpawnEmitterAtLocation` "/Game/StarterContent/Particles/P_Explosion.P_Explosion" _returnvalue_location)
  (`self.K2_DestroyActor`))

(fn `CalculateMortarVelocity`
  (returns (Velocity :type "Vector Structure"))
  (locals (TargetActorVelocity :type "Vector Structure") (TargetActorLocation :type "Vector Structure") (Arc :type "Float (double-precision)" :default 1200.0))
  (bind _target (`self.Target`))
  (set `local.TargetActorVelocity` (`self.GetVelocity` _target))
  (set `local.TargetActorLocation` (`self.K2_GetActorLocation` _target))
  (bind (_outlaunchvelocity _returnvalue) (`GameplayStatics.SuggestProjectileVelocity_CustomArc` (`self.K2_GetActorLocation`) (+ (`local.TargetActorLocation`) (* (`local.TargetActorVelocity`) (/ (`KismetMathLibrary.Vector_Distance` (`local.TargetActorLocation`) (`self.K2_GetActorLocation`)) (`KismetSystemLibrary.MakeLiteralDouble` (`local.Arc`)))))))
  (if _returnvalue
    (return _outlaunchvelocity)))

(fn `UserConstructionScript`)