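; Arrow projectile that launches on an arc toward its CurveArrowTarget, playing a release sound on spawn, or destroys itself if the target is invalid.
; On BeginPlay it computes a custom-arc launch velocity once and applies it to ProjectileMovement as a local-space velocity, with no in-flight homing.
; The aim point leads the target by its velocity scaled by distance divided by Arc.
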(event `self.ReceiveBeginPlay`
  (`/Engine/EditorBlueprintResources/StandardMacros.IsValid` (`self.curveArrowTarget`)
    (:`Is Valid`
      (`GameplayStatics.PlaySoundAtLocation` "/Game/SoundEffect/SW_Arrow/SW_ArrowRelease.SW_ArrowRelease" (`self.K2_GetActorLocation` self) (struct) 1.0 1.0 0.0 null null null null)
      (bind _velocity (`self.CalculateCurveTargetVelocity_0`))
      (`ProjectileMovementComponent.SetVelocityInLocalSpace` (`self.ProjectileMovement`) _velocity))
    (:`Is Not Valid`
      (`self.K2_DestroyActor`))))

(fn `CalculateCurveTargetVelocity_0`
  (returns (Velocity :type "Vector Structure"))
  (locals (TargetActorVelocity :type "Vector Structure") (TargetActorLocation :type "Vector Structure") (Arc :type "Float (double-precision)" :default 1200.0))
  (bind _curvearrowtarget (`self.curveArrowTarget`))
  (set `local.TargetActorVelocity` (`self.GetVelocity` _curvearrowtarget))
  (set `local.TargetActorLocation` (`self.K2_GetActorLocation` _curvearrowtarget))
  (bind (_outlaunchvelocity _returnvalue) (`GameplayStatics.SuggestProjectileVelocity_CustomArc` (`self.K2_GetActorLocation`) (+ (`local.TargetActorLocation`) (* (`local.TargetActorVelocity`) (/ (`KismetMathLibrary.Vector_Distance` (`local.TargetActorLocation`) (`self.K2_GetActorLocation`)) (`KismetSystemLibrary.MakeLiteralDouble` (`local.Arc`)))))))
  (if _returnvalue
    (return _outlaunchvelocity)))

(fn `UserConstructionScript`
  (`parent.UserConstructionScript`))