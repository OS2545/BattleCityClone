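; Player bullet actor that explodes on impact and can pass through a wall when the player has special ammo.
; On BeginPlay it reads the player character's special ammo and, if present, sets its box collision to overlap all channels.
; Overlapping walls tagged destructible or indestructible lets it through, then ending overlap restores blocking and consumes special ammo.
; Other overlaps or any hit fire a radial impulse, spawn an explosion and destroy it.
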(event `self.ReceiveBeginPlay`
  ; Check if has special bullet
  (bind _asbp_third_person_character (cast `/Game/ThirdPerson/Blueprints/BP_ThirdPersonCharacter` (`GameplayStatics.GetPlayerPawn` 0)))
  (bind _has_special_ammo_ (`/Game/ThirdPerson/Blueprints/BP_ThirdPersonCharacter.HasSpecialAmmo` _asbp_third_person_character))
  (if _has_special_ammo_
    (`PrimitiveComponent.SetCollisionResponseToAllChannels` (`self.Box`) "ECR_Overlap")))

(event `self.Box.OnComponentEndOverlap`
  (params (OverlappedComponent :type "PrimitiveComponent Object Reference") (OtherActor :type "Actor Object Reference") (OtherComp :type "PrimitiveComponent Object Reference") (OtherBodyIndex :type Integer))
  ; Has special bullet => pass throught a wall
  (if (not (`self.bulletIsDestoryed?`))
    (`PrimitiveComponent.SetCollisionResponseToAllChannels` (`self.Box`) "ECR_Block")
    (bind _asbp_third_person_character (cast `/Game/ThirdPerson/Blueprints/BP_ThirdPersonCharacter` (`GameplayStatics.GetPlayerPawn` 0)))
    (`/Game/ThirdPerson/Blueprints/BP_ThirdPersonCharacter.UseSpecialAmmo` _asbp_third_person_character)))

(event `self.Box.OnComponentBeginOverlap`
  (params (OverlappedComponent :type "PrimitiveComponent Object Reference") (OtherActor :type "Actor Object Reference") (OtherComp :type "PrimitiveComponent Object Reference") (OtherBodyIndex :type Integer) (bFromSweep :type Boolean) (SweepResult :type "HitResult Structure (by ref)"))
  (bind (_returnvalue_location _returnvalue_rotation) (`KismetMathLibrary.BreakTransform` (`SceneComponent.GetRelativeTransform` (`self.Box`))))
  (bind _output (`|GetArrayItem` (`Actor.Tags` OtherActor)))
  ; Check if it hit the boarder / if hit the boarder, the bullet is wasted
  (if (not (or (== _output "Destrucible Wall") (== _output "Indestrucible Wall")))
    (set `self.bulletIsDestoryed?` true)
    ; Hit Actor
    (`RadialForceComponent.FireImpulse` (`self.RadialForce`) :!label _label)
    (`GameplayStatics.SpawnEmitterAtLocation` "/Game/StarterContent/Particles/P_Explosion.P_Explosion" _returnvalue_location _returnvalue_rotation)
    (`self.K2_DestroyActor`)))

(event `self.Box.OnComponentHit`
  (params (HitComponent :type "PrimitiveComponent Object Reference") (OtherActor :type "Actor Object Reference") (OtherComp :type "PrimitiveComponent Object Reference") (NormalImpulse :type "Vector Structure") (Hit :type "HitResult Structure (by ref)"))
  ; Hit Actor
  (goto _label))

(fn `UserConstructionScript`)