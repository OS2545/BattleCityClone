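; BP_DestructibleWall is a wall actor that loses health when hit by bullets and is destroyed once its HP runs out.
; The wall mesh's hit event passes the other actor to a check that looks for a configurable keyword in that actor's display name, rather than testing its class.
; Each matching hit calls Damage, which subtracts a set amount from HP and destroys the actor at zero or below.
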(event `self.wallMesh.OnComponentHit`
  (params (HitComponent :type "PrimitiveComponent Object Reference") (OtherActor :type "Actor Object Reference") (OtherComp :type "PrimitiveComponent Object Reference") (NormalImpulse :type "Vector Structure") (Hit :type "HitResult Structure (by ref)"))
  (bind _hitbybullet (`self.CheckHitbyBullet?` OtherActor))
  (if _hitbybullet
    (`self.Damage`)))

(fn `CheckHitbyBullet?`
  (params (Actor :type "Actor Object Reference"))
  (returns (hitByBullet :type Boolean))
  (locals (CheckWord :type String :default "Bullet"))
  (return (`KismetStringLibrary.Contains` (`KismetSystemLibrary.GetDisplayName` Actor) (`local.CheckWord`))))

(fn `Damage`
  (locals (danageAmount :type Integer :default 1))
  (bind _output_get (set `self.HP` (- (`self.HP`) (`local.danageAmount`))))
  (if (<= _output_get 0)
    (`self.K2_DestroyActor`))
  (return))

(fn `UserConstructionScript`)