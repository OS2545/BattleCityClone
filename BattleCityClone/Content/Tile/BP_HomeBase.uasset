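; BP_HomeBase is a base tile that loses health when hit by bullets.
; Each BP_Bullet overlapping its Cube removes one HP, then sends the new value to the HUD widget through HUD_UI.
; At one HP it spawns a fire emitter using the Cube's relative location as the world position.
; At zero or below it only prints a game-over message.
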(event `self.Cube.OnComponentBeginOverlap`
  (params (OverlappedComponent :type "PrimitiveComponent Object Reference") (OtherActor :type "Actor Object Reference") (OtherComp :type "PrimitiveComponent Object Reference") (OtherBodyIndex :type Integer) (bFromSweep :type Boolean) (SweepResult :type "HitResult Structure (by ref)"))
  (cast `/Game/Bullet/BP_Bullet` OtherActor)
  (`self.Damage`)
  (`self.UpdateBaseHPUI`))

(fn `Damage`
  (bind _output_get (set `self.HP` (- (`self.HP`) 1)))
  (if (<= _output_get 0)
    (`KismetSystemLibrary.PrintString` "Game over")
    (elif (<= _output_get 1)
      (`GameplayStatics.SpawnEmitterAtLocation` "/Game/StarterContent/Particles/P_Fire.P_Fire" (`SceneComponent.RelativeLocation` (`self.Cube`))))))

(fn `UpdateBaseHPUI`
  (bind _ashud_ui (cast `/Game/UI/HUD_UI` (`PlayerController.GetHUD` (`GameplayStatics.GetPlayerController` 0))))
  (`/Game/UI/W_UI.UpdateBaseHP_Event` (`/Game/UI/HUD_UI.UI_Ref` _ashud_ui) (`self.HP`)))

(fn `UserConstructionScript`)