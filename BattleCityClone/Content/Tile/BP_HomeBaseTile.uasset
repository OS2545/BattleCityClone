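; Home base tile that loses HP each time a BP_Arrow overlaps its Cube, acting as the lose condition of the game.
; Each hit plays an impact sound, decrements HP, pushes it to the HUD_UI widget and calls BulletHit on the arrow.
; At zero HP it triggers the game mode's game-over event; at one it spawns fire VFX and sound, using the Cube's relative location.
; BeginPlay refreshes the HP display after a short delay.
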(event `self.ReceiveBeginPlay`
  (`KismetSystemLibrary.Delay` 0.1)
  (`self.UpdateBaseHPUI`))

(event `self.Cube.OnComponentBeginOverlap`
  (params (OverlappedComponent :type "PrimitiveComponent Object Reference") (OtherActor :type "Actor Object Reference") (OtherComp :type "PrimitiveComponent Object Reference") (OtherBodyIndex :type Integer) (bFromSweep :type Boolean) (SweepResult :type "HitResult Structure (by ref)"))
  (bind _asbp_arrow (cast `/Game/Bullet/BP_Arrow` OtherActor))
  (`self.Damage`)
  (`self.UpdateBaseHPUI`)
  (`/Game/Bullet/BP_Arrow.BulletHit` _asbp_arrow))

(fn `Damage`
  (bind _relativelocation (`SceneComponent.RelativeLocation` (`self.Cube`)))
  (`GameplayStatics.PlaySoundAtLocation` "/Game/SoundEffect/SW_Arrow/SW_arrow_heavySolid_impact.SW_arrow_heavySolid_impact" (`self.K2_GetActorLocation`) (struct) 1.0 1.0 0.0 null null null null)
  ; Damage HP
  (bind _result (`/Engine/EditorBlueprintResources/StandardMacros.DecrementInt` (`self.HP`))
    (:`  `
      ; Check HP
      (if (<= _result 0)
        (bind _asbp_third_person_game_mode (cast `/Game/ThirdPerson/Blueprints/BP_ThirdPersonGameMode` (`GameplayStatics.GetGameMode`)))
        (`/Game/ThirdPerson/Blueprints/BP_ThirdPersonGameMode.ED_GameOver_Event` _asbp_third_person_game_mode)
        (else
          ;; When HP <= 1 ;Spawn VFX
          (if (<= _result 1)
            (`GameplayStatics.SpawnEmitterAtLocation` "/Game/StarterContent/Particles/P_Fire.P_Fire" _relativelocation)
            (`GameplayStatics.PlaySoundAtLocation` "/Game/StarterContent/Audio/Fire01_Cue.Fire01_Cue" _relativelocation (struct) 1.0 1.0 0.0 null null null null)))))))

(fn `UpdateBaseHPUI`
  (bind _ashud_ui (cast `/Game/UI/HUD_UI` (`PlayerController.GetHUD` (`GameplayStatics.GetPlayerController` 0))))
  (`/Game/UI/W_UI.UpdateBaseHP_Event` (`/Game/UI/HUD_UI.UI_Ref` _ashud_ui) (`self.HP`)))

(fn `UserConstructionScript`)