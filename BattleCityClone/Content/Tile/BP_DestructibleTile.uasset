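; BP_DestructibleTile is a destructible wall tile whose height reflects its remaining HP.
; Arrow hits on the wall mesh call Damage, which plays an impact sound, spawns wood splatter, reduces HP, then notifies the arrow.
; SetWallMeshHeight runs on BeginPlay and after each hit, rescaling and repositioning the mesh vertically from HP.
; At zero HP the tile destroys itself, spawning a final splatter on Destroyed.
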(event `self.ReceiveBeginPlay`
  (`self.SetWallMeshHeight`))

(event `self.wallMesh.OnComponentHit`
  (params (HitComponent :type "PrimitiveComponent Object Reference") (OtherActor :type "Actor Object Reference") (OtherComp :type "PrimitiveComponent Object Reference") (NormalImpulse :type "Vector Structure") (Hit :type "HitResult Structure (by ref)"))
  (bind _asbp_arrow (cast `/Game/Bullet/BP_Arrow` OtherActor))
  (`self.Damage`)
  (`/Game/Bullet/BP_Arrow.BulletHit` _asbp_arrow))

(event `self.ReceiveDestroyed`
  (bind (_returnvalue_x _returnvalue_y _returnvalue_z) (`KismetMathLibrary.BreakVector` (`SceneComponent.K2_GetComponentLocation` (`self.wallMesh`))))
  (`NiagaraFunctionLibrary.SpawnSystemAtLocation` "/Game/VFX/WoodSplatter/NS_WoodSplatter.NS_WoodSplatter" (`KismetMathLibrary.MakeVector` _returnvalue_x _returnvalue_y _returnvalue_z)))

(fn `Damage`
  (locals (danageAmount :type Integer :default 1))
  (bind (_returnvalue_x _returnvalue_y _returnvalue_z) (`KismetMathLibrary.BreakVector` (`SceneComponent.K2_GetComponentLocation` (`self.wallMesh`))))
  ; VFX emitter
  (`GameplayStatics.PlaySoundAtLocation` "/Game/SoundEffect/SW_Arrow/SW_arrow_wood_impact.SW_arrow_wood_impact" (`self.K2_GetActorLocation`) (struct) 1.0 1.0 0.0 null null null null)
  (`NiagaraFunctionLibrary.SpawnSystemAtLocation` "/Game/VFX/WoodSplatter/NS_WoodSplatter.NS_WoodSplatter" (`KismetMathLibrary.MakeVector` _returnvalue_x _returnvalue_y (/ _returnvalue_z 2.0)))
  ; Damage HP
  (set `self.HP` (- (`self.HP`) (`local.danageAmount`)))
  (`self.SetWallMeshHeight`)
  ; Check HP
  (if (<= (`self.HP`) 0)
    (`self.K2_DestroyActor`))
  (return))

(fn `SetWallMeshHeight`
  (bind _wallmesh (`self.wallMesh`))
  (bind _wallmesh_2 (`self.wallMesh`))
  (bind (_relativescale3d_x _relativescale3d_y) (`KismetMathLibrary.BreakVector` (`SceneComponent.RelativeScale3D` _wallmesh_2)))
  (bind (_relativelocation_x _relativelocation_y) (`KismetMathLibrary.BreakVector` (`SceneComponent.RelativeLocation` _wallmesh)))
  (bind _returnvalue (* (- (`self.HP`) 1) (`self.HeightMultipleAmount`)))
  (`SceneComponent.SetRelativeScale3D` _wallmesh_2 (`KismetMathLibrary.MakeVector` _relativescale3d_x _relativescale3d_y (+ 1.0 _returnvalue)))
  (`SceneComponent.K2_SetRelativeLocation` _wallmesh (`KismetMathLibrary.MakeVector` _relativelocation_x _relativelocation_y (+ 50.0 (* _returnvalue 50.0))) false true))

(fn `UserConstructionScript`)